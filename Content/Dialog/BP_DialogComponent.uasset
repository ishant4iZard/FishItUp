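; Dialog component for a BP_Speaker actor that steps through a conversation one line per Talk call.
; The first call creates a WBP_Dialog widget with the speaker name and text, and later calls update it.
; Data table rows work as a linked list, each supplying the next row, its table and an end flag.
; Once that flag is set, the next Talk removes the widget and calls ChangeTopic on the owner.
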(event `self.ReceiveBeginPlay`)

(event `/Game/Dialog/BP_Interact.Talk`
  (params (Player :type "/Game/Pawn/BPFishingDude Object Reference"))
  (if (`self.EndDialog`)
    (`Widget.RemoveFromParent` (`self.Dialog Widget`))
    (set `self.EndDialog` false)
    (set `self.Dialog Widget` null)
    (bind _asbp_speaker (cast `/Game/Dialog/BP_Speaker` (`self.GetOwner`)))
    (`/Game/Dialog/BP_Speaker.Change topic` _asbp_speaker)
    (else
      (`/Engine/EditorBlueprintResources/StandardMacros.IsValid` (`self.Dialog Widget`)
        (:`Is Valid`
          (bind _returnvalue (`|GetDataTableRow` (`self.Dialog Data Table`) (`self.Row Name`))
            (:`then`
              (bind (_dialog _drow _datatable _benddialog) (break `/Game/Dialog/DialogStruct` _returnvalue))
              (`/Game/Dialog/UI/WBP_Dialog.Update Dialogue` (`self.Dialog Widget`) _dialog)
              (set `self.Row Name` _drow)
              (set `self.Dialog Data Table` _datatable)
              (set `self.EndDialog` _benddialog))))
        (:`Is Not Valid`
          (bind _returnvalue_2 (`|GetDataTableRow` (`self.Dialog Data Table`) (`self.Row Name`))
            (:`then`
              (bind (_dialog_2 _drow_2 _datatable_2 _benddialog_2) (break `/Game/Dialog/DialogStruct` _returnvalue_2))
              (bind _returnvalue_3 (`|CreateWidget` "/Game/Dialog/UI/WBP_Dialog.WBP_Dialog_C" null (`KismetTextLibrary.Conv_NameToText` (`self.Name`)) _dialog_2))
              (bind _output_get (set `self.Dialog Widget` _returnvalue_3))
              (`UserWidget.AddToViewport` _output_get 0)
              (`UserWidget.AddToViewport` _returnvalue_3 0)
              (set `self.Row Name` _drow_2)
              (set `self.Dialog Data Table` _datatable_2)
              (set `self.EndDialog` _benddialog_2))))))))