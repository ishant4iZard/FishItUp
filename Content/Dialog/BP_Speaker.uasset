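; BP_Speaker drives the dialog in the fishing game, starting a conversation with the BPFishingDude player shortly after BeginPlay.
; Each finished dialog queues the next topic on a fixed delay, while a DoOnce shows the player's fishing alert after the first.
; PickRandomTopic steps through AllConversation sequentially despite its name, without a bounds check.
; FinalTopic swaps in the ending dialog table but is not called within this Blueprint.
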(event `self.ReceiveBeginPlay`
  (bind _returnvalue (`GameplayStatics.GetActorOfClass` "/Game/Pawn/BPFishingDude.BPFishingDude_C"))
  (set `self.Player` _returnvalue)
  (`KismetSystemLibrary.Delay` 2.0)
  (`self.StartTalk`)
  (add `/Game/Dialog/BP_DialogComponent.DialogFinished` (`self.BP_DialogComponent`) (delegate `EndTalk`))
  (set `self.CanEnd` true))

(event `EndTalk`
  (`|ExecutionSequence`
    (:`then_0`
      (`/Engine/EditorBlueprintResources/StandardMacros.DoOnce` false
        (:`Completed`
          (`FishingCharacter.ShowFisingAlert` (`self.Player`)))))
    (:`then_1`
      (`self.WaitForNextConversation`))))

(event `StartTalk`
  (set `/Game/Pawn/BPFishingDude.InDialog` true (`self.Player`))
  (`/Game/Dialog/BP_Interact.Talk` (`self.BP_DialogComponent`) null))

(event `Change topic`
  (bind _bp_dialogcomponent (`self.BP_DialogComponent`))
  (bind _newtopic (`self.PickRandomTopic`))
  (set `/Game/Dialog/BP_DialogComponent.Dialog Data Table` _newtopic _bp_dialogcomponent)
  (set `/Game/Dialog/BP_DialogComponent.Row Name` "1" _bp_dialogcomponent)
  (`KismetSystemLibrary.Delay` 20.0)
  (`self.StartTalk`))

(event `FinalTopic`
  (bind _bp_dialogcomponent (`self.BP_DialogComponent`))
  (set `/Game/Dialog/BP_DialogComponent.Dialog Data Table` "/Game/Dialog/AllDialog/EndingDialog.EndingDialog" _bp_dialogcomponent)
  (set `/Game/Dialog/BP_DialogComponent.Row Name` "1" _bp_dialogcomponent)
  (`self.StartTalk`))

(event `WaitForNextConversation`
  (`self.Change topic`))

(fn `PickRandomTopic`
  (returns (NewTopic :type "DataTable Object Reference"))
  (bind _output_get (set `self.CurrentTopic` (+ (`self.CurrentTopic`) 1)))
  (return (`|GetArrayItem` (`self.AllConversation`) _output_get)))

(fn `UserConstructionScript`)