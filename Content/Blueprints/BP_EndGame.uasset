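; BP_EndGame is a trigger-box actor that marks where the fishing character (BPFishingDude) is allowed to end the game.
; On overlap begin it copies its own CanEnd flag onto the character, and on overlap end it resets the character's flag to false.
; Logic to show and hide an EndTip prompt is present but disconnected, so it never runs.
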(event `self.ReceiveBeginPlay`)

(event `self.Box.OnComponentBeginOverlap`
  (params (OverlappedComponent :type "PrimitiveComponent Object Reference") (OtherActor :type "Actor Object Reference") (OtherComp :type "PrimitiveComponent Object Reference") (OtherBodyIndex :type Integer) (bFromSweep :type Boolean) (SweepResult :type "HitResult Structure (by ref)"))
  (`KismetSystemLibrary.IsObjectOfSoftClass` OtherActor "/Game/Pawn/BPFishingDude.BPFishingDude_C"
    (:`True`
      (bind _asbpfishing_dude (cast `/Game/Pawn/BPFishingDude` OtherActor))
      (bind _output_get (set `/Game/Pawn/BPFishingDude.bCanEnd` (`self.bCanEnd`) _asbpfishing_dude)))))

(event `self.Box.OnComponentEndOverlap`
  (params (OverlappedComponent :type "PrimitiveComponent Object Reference") (OtherActor :type "Actor Object Reference") (OtherComp :type "PrimitiveComponent Object Reference") (OtherBodyIndex :type Integer))
  (`KismetSystemLibrary.IsObjectOfSoftClass` OtherActor "/Game/Pawn/BPFishingDude.BPFishingDude_C"
    (:`True`
      (bind _asbpfishing_dude (cast `/Game/Pawn/BPFishingDude` OtherActor))
      (set `/Game/Pawn/BPFishingDude.bCanEnd` false _asbpfishing_dude))))

(fn `UserConstructionScript`)