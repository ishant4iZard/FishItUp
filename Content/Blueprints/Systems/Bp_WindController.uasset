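; Wind controller actor that publishes wind settings to the WindParColl Material Parameter Collection.
; Its construction script writes the actor's forward vector as wind direction, along with strength and minimum and maximum wind length.
; An arrow component scales with wind strength to visualize it.
; All updates happen at construction, with no runtime event logic.
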(fn `UserConstructionScript`
  (bind _windstrength (`self.WindStrength`))
  (`KismetMaterialLibrary.SetVectorParameterValue` "/Game/Blueprints/Systems/WindParColl.WindParColl" "WindDir" (`KismetMathLibrary.Conv_VectorToLinearColor` (`self.GetActorForwardVector`)))
  (set `ArrowComponent.ArrowLength` (* _windstrength 80.0) (`self.Arrow`))
  (`KismetMaterialLibrary.SetScalarParameterValue` "/Game/Blueprints/Systems/WindParColl.WindParColl" "WindStrength" _windstrength)
  (`KismetMaterialLibrary.SetScalarParameterValue` "/Game/Blueprints/Systems/WindParColl.WindParColl" "WindLengthMin" (`self.WindLenMin`))
  (`KismetMaterialLibrary.SetScalarParameterValue` "/Game/Blueprints/Systems/WindParColl.WindParColl" "WindLengthMax" (`self.WindLenMax`)))